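; BP_DirLight drives a directional light through a timed half-turn arc, apparently a sun or moon sweep, starting at BeginPlay.
; The Coucher event resets the rotation, picks a color temperature from the Matin flag, then lerps the rotation with a timeline.
; When a sweep finishes with Matin set, it clears the flag and replays; otherwise it only casts to the player character, with no further action.
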(event `self.ReceiveBeginPlay`
  (`self.Coucher`))

(event `Coucher`
  (`SceneComponent.K2_SetWorldRotation` (`self.DirectionalLight`) (struct :`Pitch` 190.0 :`Yaw` 180.0) false false)
  (`LightComponent.SetTemperature` (`self.DirectionalLight`) (`KismetMathLibrary.SelectFloat` 11000.0 4500.0 (`self.Matin?`)))
  (bind (_direction _newtrack_0) (`Timeline|Timeline_0` :!via `PlayFromStart`)
    (:`Update`
      (`SceneComponent.K2_SetWorldRotation` (`self.DirectionalLight`) (`KismetMathLibrary.RLerp` (struct :`Pitch` 190.0 :`Yaw` 180.0) (struct :`Pitch` 370.0 :`Yaw` 180.0) _newtrack_0) false false))
    (:`Finished`
      (if (`self.Matin?`)
        (set `self.Matin?` false)
        (`self.Coucher`)
        (else
          (cast `/Game/BP/BP_ThirdPersonCharacter` (`Controller.K2_GetPawn` (`GameplayStatics.GetPlayerController` 0))))))))

(fn `UserConstructionScript`)