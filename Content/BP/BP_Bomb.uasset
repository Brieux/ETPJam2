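; Falling bomb actor that marks the ground below with a decal on BeginPlay via a downward trace, then explodes on its first mesh hit.
; Boom hides the mesh, swaps trail for explosion Niagara, shakes nearby cameras and calls Exploded on the first BP_ThirdPersonCharacter in a sphere trace.
; A delayed explosion sound follows, and the actor destroys itself when the effect finishes.
; The drop-sound setup is unwired, though Boom still stops it.
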(event `self.ReceiveBeginPlay`
  (bind _returnvalue (`self.K2_GetActorLocation`))
  (bind _outhit (`KismetSystemLibrary.LineTraceSingle` :`Start` _returnvalue :`End` (+ (* (`KismetMathLibrary.NegateVector` (`self.GetActorUpVector`)) 10000.0) _returnvalue) :`TraceChannel` "TraceTypeQuery2" :`DrawDebugType` "Persistent"))
  (`GameplayStatics.SpawnDecalAtLocation` "/Game/OmbreBombr_Mat.OmbreBombr_Mat" (100.0 100.0 100.0) (`.Location` (`GameplayStatics.BreakHitResult` _outhit)) (`KismetMathLibrary.Conv_VectorToRotator` (`.ImpactNormal` (`GameplayStatics.BreakHitResult` _outhit)))))

(event `self.StaticMesh.OnComponentHit`
  (params (HitComponent :type "PrimitiveComponent Object Reference") (OtherActor :type "Actor Object Reference") (OtherComp :type "PrimitiveComponent Object Reference") (NormalImpulse :type "Vector Structure") (Hit :type "HitResult Structure (by ref)"))
  (`/Engine/EditorBlueprintResources/StandardMacros.DoOnce` false
    (:`Completed`
      (`self.Boom`))))

(event `Boom`
  (bind _returnvalue (`self.K2_GetActorLocation`))
  (`AudioComponent.Stop` (`self.NewVar_0`))
  (`SceneComponent.SetVisibility` (`self.StaticMesh`) false false)
  (`ActorComponent.Deactivate` (`self.NS_BombTrail`))
  (`ActorComponent.Activate` (`self.Niagara`) false)
  (`GameplayStatics.PlayWorldCameraShake` "/Game/BP/BP_Cam_Shake_Bomb.BP_Cam_Shake_Bomb_C" (`self.K2_GetActorLocation`) 400.0 2000.0 2.0 true)
  (bind _outhits (`KismetSystemLibrary.SphereTraceMulti` :`Start` _returnvalue :`End` _returnvalue :`Radius` (`self.BombRadius`) :`TraceChannel` "TraceTypeQuery2" :`DrawDebugType` "Persistent"))
  (for _array_element _outhits
    (bind _asbp_third_person_character (cast `/Game/BP/BP_ThirdPersonCharacter` (`.HitActor` (`GameplayStatics.BreakHitResult` _array_element))))
    (`/Game/BP/BP_ThirdPersonCharacter.Exploded` _asbp_third_person_character true)
    (break))
  (`KismetSystemLibrary.Delay` 0.1)
  (`GameplayStatics.SpawnSoundAtLocation` "/Game/Son/Explosion_Obus_V1_Cue.Explosion_Obus_V1_Cue" (`self.K2_GetActorLocation`) (struct) 1.0 1.0 0.0 "/Game/Son/BP_Attenuation1.BP_Attenuation1" null))

(event `self.Niagara.OnSystemFinished`
  (params (PSystem :type "NiagaraComponent Object Reference"))
  (`self.K2_DestroyActor`))

(fn `UserConstructionScript`)