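; BP_BombZone is an actor that repeatedly spawns bombs within a zone sized by its Size variable.
; A looping timer started on BeginPlay moves the zone's mesh 3000 units ahead of the player along X, matching Y and keeping its height.
; Each tick of that timer spawns a BP_Bomb at a random-direction offset of Size from the actor's location.
; The construction script scales the mesh from Size to represent the zone.
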(event `self.ReceiveBeginPlay`
  (`KismetSystemLibrary.K2_SetTimerDelegate` (delegate `DropBomb`) (`self.Time`) true))

(event `DropBomb`
  (bind _staticmesh (`self.StaticMesh`))
  (bind (_returnvalue_x _returnvalue_y _returnvalue_z) (`KismetMathLibrary.BreakVector` (`SceneComponent.K2_GetComponentLocation` _staticmesh)))
  (bind (_returnvalue_x_2 _returnvalue_y_2) (`KismetMathLibrary.BreakVector` (`SceneComponent.K2_GetComponentLocation` (`Character.CapsuleComponent` (`GameplayStatics.GetPlayerCharacter` 0)))))
  (`SceneComponent.K2_SetWorldLocation` _staticmesh (`KismetMathLibrary.MakeVector` (+ _returnvalue_x_2 3000.0) _returnvalue_y_2 _returnvalue_z) false false)
  (`|SpawnActorFromClass` "/Game/BP/BP_Bomb.BP_Bomb_C" (`KismetMathLibrary.MakeTransform` (+ (`self.K2_GetActorLocation`) (* (* (`KismetMathLibrary.RandomUnitVector`) (`KismetMathLibrary.SelectFloat` -1.0 1.0 (`KismetMathLibrary.RandomBool`))) (`self.Size`)))) "Undefined" "OverrideRootScale" null null))

(fn `UserConstructionScript`
  (`SceneComponent.SetWorldScale3D` (`self.StaticMesh`) (* (`self.Size`) 0.01)))