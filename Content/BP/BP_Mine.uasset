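; BP_Mine is a landmine actor that arms when the player character steps on it and explodes when they step off.
; Box begin overlap caches the BP_ThirdPersonCharacter, sets WillExplode and plays a click sound.
; Box end overlap checks that flag and calls the Boom event, which activates the NSBoom effect, plays an explosion sound and calls Exploded on the cached character.
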(event `self.ReceiveTick`
  (params (DeltaSeconds :type "Float (single-precision)")))

(event `self.Box.OnComponentBeginOverlap`
  (params (OverlappedComponent :type "PrimitiveComponent Object Reference") (OtherActor :type "Actor Object Reference") (OtherComp :type "PrimitiveComponent Object Reference") (OtherBodyIndex :type Integer) (bFromSweep :type Boolean) (SweepResult :type "HitResult Structure (by ref)"))
  (bind _asbp_third_person_character (cast `/Game/BP/BP_ThirdPersonCharacter` OtherActor))
  (set `self.WillExplode?` true)
  (set `self.As BP Third Person Character` _asbp_third_person_character)
  (`GameplayStatics.PlaySound2D` "/Game/Son/ClickMine.ClickMine" 1.0 1.0 0.0 null null))

(event `self.Box.OnComponentEndOverlap`
  (params (OverlappedComponent :type "PrimitiveComponent Object Reference") (OtherActor :type "Actor Object Reference") (OtherComp :type "PrimitiveComponent Object Reference") (OtherBodyIndex :type Integer))
  (cast `/Game/BP/BP_ThirdPersonCharacter` OtherActor)
  (if (`self.WillExplode?`)
    (`self.Boom`)))

(event `Boom`
  (`ActorComponent.Activate` (`self.NS_Boom`) false)
  (`GameplayStatics.PlaySound2D` "/Game/Son/Explosion_Obus_V2.Explosion_Obus_V2" 1.0 1.0 0.0 null null)
  (`/Game/BP/BP_ThirdPersonCharacter.Exploded` (`self.As BP Third Person Character`) false))

(fn `UserConstructionScript`)