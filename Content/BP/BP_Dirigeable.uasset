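; BP_Dirigeable is an airship actor that moves its static mesh along a spline, starting at BeginPlay.
; A timeline, with play rate scaled from the Speed variable, supplies the spline time used to set the mesh's world location and rotation on each update.
; A second timeline track then adds a vertical world offset on top of the spline position.
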(event `self.ReceiveBeginPlay`
  (bind _spline (`self.Spline`))
  (`TimelineComponent.SetPlayRate` (`self.Timeline_0`) (/ (`self.Speed`) 10.0))
  (bind (_direction _newtrack_0 _newtrack_1) (`Timeline|Timeline_0`)
    (:`Update`
      (`SceneComponent.K2_SetWorldLocationAndRotation` (`self.StaticMesh`) (`SplineComponent.GetLocationAtTime` _spline _newtrack_0 "World" false) (`SplineComponent.GetRotationAtTime` _spline _newtrack_0 "World" false) false false)
      (`SceneComponent.K2_AddWorldOffset` (`self.StaticMesh`) (`KismetMathLibrary.MakeVector` 0.0 0.0 _newtrack_1) false false))))

(fn `UserConstructionScript`)